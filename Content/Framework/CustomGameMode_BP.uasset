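; Racing game mode that runs a race from intro cinematic through countdown, pause, restart and win or lose endings, extending parent game mode events.
; BeginPlay starts fading-in music and plays the intro sequence, then loads the game and starts the HUD countdown.
; A gate opened at game start lets delayed Tick append car transforms for ghost recording.
; Dispatchers signal engine and ghost state; endings share a once-only AfterRace for UI and cinematic.
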(event `self.ReceiveBeginPlay`
  (`parent.ReceiveBeginPlay`)
  (`|ExecutionSequence`
    (:`then_0`
      (bind _assports_car_bp (cast `/Game/Vehicles/SportsCar/SportsCar_BP` (`GameplayStatics.GetPlayerPawn` 0)))
      (set `self.Car` _assports_car_bp)
      (bind _returnvalue (`GameplayStatics.SpawnSound2D` "/Game/Sound/raceMusicWAV_Cue.raceMusicWAV_Cue" 1.0 1.0 0.0 null))
      (set `self.RacingMusic` _returnvalue)
      (`AudioComponent.FadeIn` _returnvalue 10.0 0.6 0.0 "Linear"))
    (:`then_1`
      (bind _ascustom_hud (cast `/Game/Framework/CustomHUD` (`PlayerController.GetHUD` (`GameplayStatics.GetPlayerController` 0))))
      (set `self.GameHUD` _ascustom_hud)
      (bind _outactor (`LevelSequencePlayer.CreateLevelSequencePlayer` "/Game/Cinematics/BeginSequence.BeginSequence" (make `MovieSceneSequencePlaybackSettings` false (struct) 1.0 0.0 false false false true)))
      (`MovieSceneSequencePlayer.Play` (`LevelSequenceActor.SequencePlayer` _outactor))
      (`KismetSystemLibrary.Delay` (`TimeManagementBlueprintLibrary.Conv_QualifiedFrameTimeToSeconds` (`MovieSceneSequencePlayer.GetDuration` (`LevelSequenceActor.SequencePlayer` _outactor))))
      (`self.LoadGame`)
      (`self.StartGame`))))

(event `self.StartGame`
  (bind _gamehud (`self.GameHUD`))
  (`parent.StartGame`)
  (`self.EngineOn` true)
  (`/Game/Framework/CustomHUD.HideHud` _gamehud false)
  (`/Game/Framework/CustomHUD.StartCountdown` _gamehud (`self.CountdownTime`))
  (`self.UnlockGhost`))

(event `self.ReceiveTick`
  (params (DeltaSeconds :type "Float (single-precision)"))
  (`/Engine/EditorBlueprintResources/StandardMacros.Gate` true :!label _label
    (:`Exit`
      (`KismetSystemLibrary.Delay` 0.01)
      (`self.RecordGhost`))))

(event `UnlockGhost`
  (`self.GhostReady`)
  (goto _label :!via `Open`))

(event `self.StartRace`
  (`parent.StartRace`)
  (bind _ascar (cast `Car` (`GameplayStatics.GetPlayerPawn` 0)))
  (`Car.StartCar` _ascar))

(event `self.RestartGame`
  (`parent.RestartGame`)
  (`WidgetBlueprintLibrary.SetInputMode_GameOnly` (`GameplayStatics.GetPlayerController` 0) true)
  (`GameplayStatics.SetGamePaused` false)
  (bind _returnvalue (`GameplayStatics.GetCurrentLevelName` true))
  (`KismetSystemLibrary.Delay` 1.0)
  (`GameplayStatics.OpenLevel` (`KismetStringLibrary.Conv_StringToName` _returnvalue)))

(event `self.ResumeGame`
  (bind _pausemusic (`self.PauseMusic`))
  (`parent.ResumeGame`)
  (`AudioComponent.Stop` _pausemusic)
  (`ActorComponent.K2_DestroyComponent` _pausemusic)
  (`AudioComponent.SetPaused` (`self.RacingMusic`) false)
  (`self.EngineOn` true)
  (`WidgetBlueprintLibrary.SetInputMode_GameOnly` (`GameplayStatics.GetPlayerController` 0) true)
  (`GameplayStatics.SetGamePaused` false)
  (`/Game/Framework/CustomHUD.OnResumeGame` (`self.GameHUD`)))

(event `self.PauseGame`
  (`parent.PauseGame`)
  (bind _returnvalue (`GameplayStatics.SpawnSound2D` "/Game/Sound/racingPauseWAV_Cue.racingPauseWAV_Cue" 1.0 1.0 0.0 null))
  (set `self.PauseMusic` _returnvalue)
  (`AudioComponent.SetPaused` (`self.RacingMusic`) true)
  (`self.EngineOn` false)
  (`WidgetBlueprintLibrary.SetInputMode_GameAndUIEx` (`GameplayStatics.GetPlayerController` 0) null)
  (`GameplayStatics.SetGamePaused` true)
  (`/Game/Framework/CustomHUD.OnPauseGame` (`self.GameHUD`)))

(event `self.QuittoMenu`
  (bind _returnvalue (`GameplayStatics.GetPlayerController` 0))
  (`WidgetBlueprintLibrary.SetInputMode_GameAndUIEx` _returnvalue null "DoNotLock" true true)
  (set `PlayerController.bShowMouseCursor` true _returnvalue)
  (`GameplayStatics.OpenLevel` "MenuLevel"))

(event `self.FinishGame`
  (`parent.FinishGame`)
  (set `self.WON` true)
  (bind _outactor (`LevelSequencePlayer.CreateLevelSequencePlayer` "/Game/Cinematics/EndSequence/WinSequence.WinSequence" (make `MovieSceneSequencePlaybackSettings` false (struct) 1.0 0.0 false true false true false false false true)))
  (set `self.Sequence` _outactor)
  (`self.AfterRace`))

(event `self.LoseGame`
  (`parent.LoseGame`)
  (`KismetSystemLibrary.Delay` 3.0)
  (bind _outactor (`LevelSequencePlayer.CreateLevelSequencePlayer` "/Game/Cinematics/EndSequence/LoseSequence.LoseSequence" (make `MovieSceneSequencePlaybackSettings` false (struct) 1.0 0.0 false true false true false false false true)))
  (set `self.Sequence` _outactor)
  (`self.AfterRace`))

(event `AfterRace`
  (bind _returnvalue (`GameplayStatics.GetPlayerController` 0))
  (`/Engine/EditorBlueprintResources/StandardMacros.DoOnce` false
    (:`Completed`
      (`self.EngineOn` false)
      (`WidgetBlueprintLibrary.SetInputMode_UIOnlyEx` _returnvalue null "DoNotLock" true)
      (set `PlayerController.bShowMouseCursor` true _returnvalue)
      (`/Game/Framework/CustomHUD.EndGameUI` (`self.GameHUD`))
      (`MovieSceneSequencePlayer.Play` (`LevelSequenceActor.SequencePlayer` (`self.Sequence`))))))

(event `ShowScores`
  (`/Game/Framework/CustomHUD.ShowScores` (`self.GameHUD`)))

(event `ClearScores`
  (`/Game/Framework/CustomHUD.EndGameUI` (`self.GameHUD`)))

(fn `LoadGame`
  (`parent.LoadGame`))

(fn `RecordGhost`
  (locals (index :type Integer :default 1))
  (`KismetArrayLibrary.Array_Add` (`self.GhostRecord`) (`self.GetTransform` (`self.Car`))))

(fn `UserConstructionScript`)