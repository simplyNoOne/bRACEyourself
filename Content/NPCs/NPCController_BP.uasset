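; NPC controller Blueprint that moves its NPC along a spline path over a requested duration.
; WalkPath sets the Following timeline's play rate to the inverse of Duration, then plays it.
; Each update maps the timeline's Alpha to a distance along PathToFollow and issues MoveToLocation to that world point with pathfinding disabled, so the NPC chases a moving target on the spline.
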(event `self.WalkPath`
  (params (Duration :type "Float (single-precision)"))
  (bind _output_get (set `self.Duration` Duration))
  (`TimelineComponent.SetPlayRate` (`self.Following`) (/ 1.0 _output_get))
  (bind (_direction _alpha) (`Timeline|Following`)
    (:`Update`
      (set `self.Alpha` _alpha)
      (`self.MoveToLocation` (`SplineComponent.GetLocationAtDistanceAlongSpline` (`self.PathToFollow`) (`KismetMathLibrary.Lerp` 0.0 (`SplineComponent.GetSplineLength` (`self.PathToFollow`)) (`self.Alpha`)) "World") -1.0 true false false true null))))

(fn `UserConstructionScript`)