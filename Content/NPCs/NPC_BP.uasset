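; NPC character that gets knocked over by cars and removes itself afterwards.
; Sets its walk speed on BeginPlay, then watches its Range component for hits or overlaps from actors implementing CarInterface.
; Either contact enables physics on the capsule and mesh and starts a timer that destroys the NPC seconds later.
; The overlap path fires once and also sends NPChitMessage to the car; SetThePath is an empty stub.
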(event `self.ReceiveBeginPlay`
  (set `CharacterMovementComponent.MaxWalkSpeed` (`self.MovementSpeed`) (`self.CharacterMovement`)))

(event `self.Range.OnComponentHit`
  (params (HitComponent :type "PrimitiveComponent Object Reference") (OtherActor :type "Actor Object Reference") (OtherComp :type "PrimitiveComponent Object Reference") (NormalImpulse :type "Vector Structure") (Hit :type "HitResult Structure (by ref)"))
  (if (`KismetSystemLibrary.DoesImplementInterface` OtherActor "/Script/bRACEyourself.CarInterface")
    (`PrimitiveComponent.SetCollisionEnabled` (`self.CapsuleComponent`) "QueryAndPhysics")
    (`PrimitiveComponent.SetCollisionEnabled` (`self.Mesh`) "QueryAndPhysics")
    (`PrimitiveComponent.SetSimulatePhysics` (`self.Mesh`) true)
    (`PrimitiveComponent.SetSimulatePhysics` (`self.CapsuleComponent`) true)
    (bind _returnvalue (`KismetSystemLibrary.K2_SetTimerDelegate` (delegate `Destroy`) 6.0))))

(event `SetThePath`)

(event `Destroy`
  (`self.K2_DestroyActor`)
  (`KismetSystemLibrary.K2_ClearAndInvalidateTimerHandle` (stale `self.Range.OnComponentHit` _returnvalue)))

(event `self.Range.OnComponentBeginOverlap`
  (params (OverlappedComponent :type "PrimitiveComponent Object Reference") (OtherActor :type "Actor Object Reference") (OtherComp :type "PrimitiveComponent Object Reference") (OtherBodyIndex :type Integer) (bFromSweep :type Boolean) (SweepResult :type "HitResult Structure (by ref)"))
  (if (`KismetSystemLibrary.DoesImplementInterface` OtherActor "/Script/bRACEyourself.CarInterface")
    (`/Engine/EditorBlueprintResources/StandardMacros.DoOnce` false
      (:`Completed`
        (`KismetSystemLibrary.PrintString` "Hello")
        (message `CarInterface.NPChit` OtherActor)
        (`PrimitiveComponent.SetCollisionEnabled` (`self.CapsuleComponent`) "QueryAndPhysics")
        (`PrimitiveComponent.SetCollisionEnabled` (`self.Mesh`) "QueryAndPhysics")
        (`PrimitiveComponent.SetSimulatePhysics` (`self.Mesh`) true)
        (`PrimitiveComponent.SetSimulatePhysics` (`self.CapsuleComponent`) true)
        (bind _returnvalue (`KismetSystemLibrary.K2_SetTimerDelegate` (delegate `DestoryNpc`) 6.0))))))

(event `DestoryNpc`
  (`self.K2_DestroyActor`)
  (`KismetSystemLibrary.K2_ClearAndInvalidateTimerHandle` (stale `self.Range.OnComponentBeginOverlap` _returnvalue)))

(fn `UserConstructionScript`)